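; Shared multiplayer camera that keeps two to four players in frame, set as the view target for every player controller.
; After a short delay, ClassSetup reads the player list from BP_GameMode, stores and numbers each player, then a fast looping timer drives UpdateCamera.
; Per player count, it moves smoothly to the players' average location and sets spring arm length to their largest pairwise distance, clamped to min and max.
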(event Custom|UpdateCamera
  (switch int (Utilities|Array|Length (Variables|Default|GetPlayersReference))
    (:2
      (CallFunction|SetArmLength2p)
      (CallFunction|SetCameraPosP2))
    (:3
      (CallFunction|SetArmLength3P)
      (CallFunction|SetCameraPosP3))
    (:4
      (CallFunction|SetArmLength4P)
      (CallFunction|SetCameraPosP4))))

(event EventBeginPlay
  (Utilities|FlowControl|Delay 0.2)
  (CallFunction|ClassSetup)
  (Utilities|Time|SetTimerbyFunctionName 0 "UpdateCamera" 0.001 true))

(fn ConstructionScript)

(fn ClassSetup
  (bind _asbp_game_mode (Utilities|Casting|CastToBP_GameMode (Game|GetGameMode)))
  ;[1 1 1] Get the # of players spawned from the GameMode BP
  (bind _output_get (Variables|Default|SetBP_GameMode _asbp_game_mode))
  (Variables|Default|SetPlayersReference (Variables|/Game/Blueprints/BP_GameMode.BP_GameMode_C|GetPlayers _output_get))
  ;[1 1 1] Get each players player controller, set their view target to BP_Camera(SELF)
  (bind _outactors (Actor|GetAllActorsOfClass "/Script/Engine.PlayerController"))
  (Game|Player|SetViewTargetwithBlend _outactors self 0.0 "VTBlend_Linear" 0.0 false)
  (for (_array_element _array_index) (Variables|Default|GetPlayersReference)
    (switch int _array_index
      (:0
        (bind _output_get_2 (Variables|Default|SetP1 _array_element))
        (Variables|/Game/Blueprints/BP_Player.BP_Player_C|SetPlayerNumber _output_get_2 0))
      (:1
        (bind _output_get_3 (Variables|Default|SetP2 _array_element))
        (Variables|/Game/Blueprints/BP_Player.BP_Player_C|SetPlayerNumber _output_get_3 1))
      (:2
        (bind _output_get_4 (Variables|Default|SetP3 _array_element))
        (Variables|/Game/Blueprints/BP_Player.BP_Player_C|SetPlayerNumber _output_get_4 2))
      (:3
        (bind _output_get_5 (Variables|Default|SetP4 _array_element))
        (Variables|/Game/Blueprints/BP_Player.BP_Player_C|SetPlayerNumber _output_get_5 3)))))

(fn SetArmLength4P
  (bind _p1 (Variables|Default|GetP1))
  (bind _p2 (Variables|Default|GetP2))
  (bind _p3 (Variables|Default|GetP3))
  (bind _p4 (Variables|Default|GetP4))
  (Variables|/Script/Engine.SpringArmComponent|SetTargetArmLength (Variables|Default|GetSpringArm) (Math|Float|Clamp(Float) (.MaxValue (Math|Float|MaxOfFloatArray (Utilities|Array|MakeArray (Transformation|GetDistanceTo _p1 _p2) (Transformation|GetDistanceTo _p1 _p3) (Transformation|GetDistanceTo _p1 _p4) (Transformation|GetDistanceTo _p2 _p3) (Transformation|GetDistanceTo _p2 _p4) (Transformation|GetDistanceTo _p3 _p4)))) (Variables|Default|GetMinArmLength) (Variables|Default|GetMaxArmLength))))

(fn SetArmLength3P
  (bind _p1 (Variables|Default|GetP1))
  (bind _p2 (Variables|Default|GetP2))
  (bind _p3 (Variables|Default|GetP3))
  (Variables|/Script/Engine.SpringArmComponent|SetTargetArmLength (Variables|Default|GetSpringArm) (Math|Float|Clamp(Float) (.MaxValue (Math|Float|MaxOfFloatArray (Utilities|Array|MakeArray (Transformation|GetDistanceTo _p1 _p2) (Transformation|GetDistanceTo _p1 _p3) (Transformation|GetDistanceTo _p2 _p3)))) (Variables|Default|GetMinArmLength) (Variables|Default|GetMaxArmLength))))

(fn SetArmLength2p
  (Variables|/Script/Engine.SpringArmComponent|SetTargetArmLength (Variables|Default|GetSpringArm) (Math|Float|Clamp(Float) (Transformation|GetDistanceTo (Variables|Default|GetP1) (Variables|Default|GetP2)) (Variables|Default|GetMinArmLength) (Variables|Default|GetMaxArmLength))))

(fn SetCameraPosP4
  (Variables|Default|SetTargetPos (/ (+ (Transformation|GetActorLocation (Variables|Default|GetP1)) (Transformation|GetActorLocation (Variables|Default|GetP2)) (Transformation|GetActorLocation (Variables|Default|GetP3)) (Transformation|GetActorLocation (Variables|Default|GetP4))) (Math|Conversions|ToFloat(Integer) (Utilities|Array|Length (Variables|Default|GetPlayersReference)))))
  (Transformation|SetActorLocation (Math|Interpolation|VInterpTo (Variables|Default|GetPreviousPos) (Variables|Default|GetTargetPos) (Utilities|Time|GetWorldDeltaSeconds) 1e+01) false false)
  (Variables|Default|SetPreviousPos (Transformation|GetActorLocation)))

(fn SetCameraPosP3
  (Variables|Default|SetTargetPos (/ (+ (Transformation|GetActorLocation (Variables|Default|GetP1)) (Transformation|GetActorLocation (Variables|Default|GetP2)) (Transformation|GetActorLocation (Variables|Default|GetP3))) (Math|Conversions|ToFloat(Integer) (Utilities|Array|Length (Variables|Default|GetPlayersReference)))))
  (Transformation|SetActorLocation (Math|Interpolation|VInterpTo (Variables|Default|GetPreviousPos) (Variables|Default|GetTargetPos) (Utilities|Time|GetWorldDeltaSeconds) 1e+01) false false)
  (Variables|Default|SetPreviousPos (Transformation|GetActorLocation)))

(fn SetCameraPosP2
  (Variables|Default|SetTargetPos (/ (+ (Transformation|GetActorLocation (Variables|Default|GetP1)) (Transformation|GetActorLocation (Variables|Default|GetP2))) (Math|Conversions|ToFloat(Integer) (Utilities|Array|Length (Variables|Default|GetPlayersReference)))))
  (Transformation|SetActorLocation (Math|Interpolation|VInterpTo (Variables|Default|GetPreviousPos) (Variables|Default|GetTargetPos) (Utilities|Time|GetWorldDeltaSeconds) 1e+01) false false)
  (Variables|Default|SetPreviousPos (Transformation|GetActorLocation)))