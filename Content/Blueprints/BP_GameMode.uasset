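; Game mode for a local multiplayer game with three timed rounds and per-player scores for four players.
; BeginPlay spawns and possesses a BP_Player at each index-tagged PlayerStart, assigns animal meshes by index, and shows score and timer widgets.
; Delay-gated Tick counts down each round; expiry starts the next, briefly disabling input, swapping widgets and teleporting players.
; Round three covers only two players, and its end triggers nothing further.
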(event Custom|AddScoreToPlayerOne
  (params (AddP1Score :type Integer))
  ;[1 1 1] Add Score to Player One
  (Variables|Default|SetPlayerOneScore (+ AddP1Score (Variables|Default|GetPlayerOneScore))))

(event Custom|AddScoreToPlayerTwo
  (params (AddP2Score :type Integer))
  ;[1 1 1] Add Score to Player Two
  (Variables|Default|SetPlayerTwoScore (+ AddP2Score (Variables|Default|GetPlayerTwoScore))))

(event Custom|RoundTwo
  (bind _returnvalue (Game|GetPlayerController 0))
  ;[1 1 1] Start round two event
  (if (Variables|Default|GetRoundOneComplete)
    (bind _returnvalue_2 (UserInterface|CreateWidget "/Game/UI/RoundTwoStart.RoundTwoStart_C"))
    (UserInterface|Viewport|AddtoViewport _returnvalue_2 0)
    (Utilities|FlowControl|Sequence
      (:then_0
        (Input|DisableInput (Game|GetPlayerCharacter 0) (Game|GetPlayerController 0)))
      (:then_1
        (Input|DisableInput (Game|GetPlayerCharacter 1) (Game|GetPlayerController 1)))
      (:then_2
        (Input|DisableInput (Game|GetPlayerCharacter 2) (Game|GetPlayerController 2)))
      (:then_3
        (Input|DisableInput (Game|GetPlayerCharacter 3) (Game|GetPlayerController 3))))
    (Utilities|FlowControl|Delay 2.0)
    (Widget|RemovefromParent _returnvalue_2)
    (Utilities|FlowControl|Sequence
      (:then_0
        (Input|EnableInput (Game|GetPlayerCharacter 0) _returnvalue)
        (Transformation|Teleport (Game|Player|GetPlayerPawn 0) "0, 0, 0" "0, 0, 0"))
      (:then_1
        (Input|EnableInput (Game|GetPlayerCharacter 1) (Game|GetPlayerController 1))
        (Transformation|Teleport (Game|Player|GetPlayerPawn 1) "1.000000, 0, 0" "0, 0, 0")
        (bind _returnvalue_3 (UserInterface|CreateWidget "/Game/Blueprints/TimerUI2.TimerUI2_C" _returnvalue))
        (UserInterface|Viewport|AddtoViewport _returnvalue_3 0))
      (:then_2
        (Input|EnableInput (Game|GetPlayerCharacter 2) (Game|GetPlayerController 2))
        (Transformation|Teleport (Game|Player|GetPlayerPawn 2) "0, 0, 0" "0, 0, 0"))
      (:then_3
        (Input|EnableInput (Game|GetPlayerCharacter 3) (Game|GetPlayerController 3))
        (Transformation|Teleport (Game|Player|GetPlayerPawn 3) "0, 0, 0" "0, 0, 0")))))

(event Custom|RoundThree
  (bind _returnvalue (Game|GetPlayerController 0))
  ;[1 1 1] Round THree Custom Event
  (if (Variables|Default|GetRoundTwoComplete)
    (bind _returnvalue_2 (UserInterface|CreateWidget "/Game/UI/RoundThreeStart.RoundThreeStart_C"))
    (UserInterface|Viewport|AddtoViewport _returnvalue_2 0)
    (Utilities|FlowControl|Sequence
      (:then_0
        (Input|DisableInput (Game|GetPlayerCharacter 0) (Game|GetPlayerController 0)))
      (:then_1
        (Input|DisableInput (Game|GetPlayerCharacter 1) (Game|GetPlayerController 1))))
    (Utilities|FlowControl|Delay 2.0)
    (Widget|RemovefromParent _returnvalue_2)
    (Utilities|FlowControl|Sequence
      (:then_0
        (Input|EnableInput (Game|GetPlayerCharacter 0) _returnvalue)
        (Transformation|Teleport (Game|Player|GetPlayerPawn 0) "0, 0, 0" "0, 0, 0"))
      (:then_1
        (Input|EnableInput (Game|GetPlayerCharacter 1) (Game|GetPlayerController 1))
        (Transformation|Teleport (Game|Player|GetPlayerPawn 1) "2.000000, 0, 0" "0, 0, 0")
        (bind _returnvalue_3 (UserInterface|CreateWidget "/Game/Blueprints/TimerUI3.TimerUI3_C" _returnvalue))
        (UserInterface|Viewport|AddtoViewport _returnvalue_3 0)))))

(event Custom|AddScoreToPlayerThree
  (params (AddP3Score :type Integer))
  ;[1 1 1] Add Score to player three
  (Variables|Default|SetPlayerThreeScore (+ AddP3Score (Variables|Default|GetPlayerThreeScore))))

(event Custom|AddScoreToPlayerFour
  (params (AddP4Score :type Integer))
  ;[1 1 1] Add Score to player four
  (Variables|Default|SetPlayerFourScore (+ AddP4Score (Variables|Default|GetPlayerFourScore))))

(event EventBeginPlay
  (Utilities|FlowControl|Sequence
    (:then_0
      (CallFunction|GetPlayerStartPoints)
      (CallFunction|SpawnPlayers))
    (:then_1
      (bind _returnvalue (UserInterface|CreateWidget "/Game/Blueprints/PointUI.PointUI_C" (Game|GetPlayerController 0)))
      (bind _returnvalue_2 (UserInterface|CreateWidget "/Game/Blueprints/TimerUI.TimerUI_C" (Game|GetPlayerController 0)))
      (UserInterface|Viewport|AddtoViewport _returnvalue_2 0))))

(event EventTick
  (params (DeltaSeconds :type Float%20%28single-precision%29))
  ;[1 1 1] Event Tick to run the timers. WIll fix
  (Utilities|FlowControl|Sequence
    (:then_0
      (Utilities|FlowControl|Delay 1.0)
      (CallFunction|RunTimer))
    (:then_1
      (if (Variables|Default|GetRoundOneComplete)
        (Utilities|FlowControl|Delay 1.0)
        (CallFunction|RunTimerTwo)))
    (:then_2
      (if (Variables|Default|GetRoundTwoComplete)
        (Utilities|FlowControl|Delay 1.0)
        (CallFunction|RunTimerThree)))))

(fn ConstructionScript)

(fn GetPlayerStartPoints
  (bind _outactors (Actor|GetAllActorsOfClass "/Script/Engine.PlayerStart"))
  (Variables|Default|SetPlayerStartArray _outactors))

(fn SpawnPlayers
  ;[0.4158 1 0.9701] Array is zero based, update for normal 1-4 use.
  (for _index (range 0 (- (Variables|Default|GetMaxPlayerCount) 1))
    (Variables|Default|SetIndex _index)
    ;[0.4374 1 0.9901] Assign each player from the array with the player start tag
    (for _array_element (Variables|Default|GetPlayerStartArray)
      (if (Utilities|Name|Equal(Name) (Variables|/Script/Engine.PlayerStart|GetPlayerStartTag _array_element) (Utilities|String|StringToName (Utilities|String|ToString(Integer) (Variables|Default|GetIndex))))
        ;[0.4256 1 0.9602] Spawn the BP_Player and assign the player to posses it
        (Class|GameplayStatics|CreatePlayer (Variables|Default|GetIndex))
        (bind _returnvalue (Game|SpawnActorfromClass "/Game/Blueprints/BP_Player.BP_Player_C" (Transformation|GetActorTransform _array_element) "Undefined" 0 0))
        (Pawn|Possess (Game|GetPlayerController (Variables|Default|GetIndex)) _returnvalue)
        ;[1 1 1] Add each unique element to the players array
        (Utilities|Array|AddUnique (Variables|Default|GetPlayers) _returnvalue)
        ;[0.2696 0.9602 1] Change the mesh and animations based on player index
        (switch int (Variables|Default|GetIndex)
          (:0
            (Class|SkinnedMeshComponent|SetSkeletalMesh (Variables|/Script/Engine.Character|GetMesh _returnvalue) "/Game/Assets/Animations/Bear/Bear_IdleAnim.Bear_IdleAnim" true)
            (Components|SkeletalMesh|SetAnimInstanceClass (Variables|/Script/Engine.Character|GetMesh _returnvalue) "/Game/Assets/Animations/Bear/BearAnimBP.BearAnimBP_C"))
          (:1
            (Class|SkinnedMeshComponent|SetSkeletalMesh (Variables|/Script/Engine.Character|GetMesh _returnvalue) "/Game/Assets/Animations/Fox/Fox_IdleAnim.Fox_IdleAnim" true)
            (Components|SkeletalMesh|SetAnimInstanceClass (Variables|/Script/Engine.Character|GetMesh _returnvalue) "/Game/Assets/Animations/Fox/Fox_ANIM_BP.Fox_ANIM_BP_C"))
          (:2
            (Class|SkinnedMeshComponent|SetSkeletalMesh (Variables|/Script/Engine.Character|GetMesh _returnvalue) "/Game/Assets/Animations/Penguin/Penguin_IdleAnim.Penguin_IdleAnim" true)
            (Components|SkeletalMesh|SetAnimInstanceClass (Variables|/Script/Engine.Character|GetMesh _returnvalue) "/Game/Assets/Animations/Penguin/PenguinBP.PenguinBP_C"))
          (:3
            (Class|SkinnedMeshComponent|SetSkeletalMesh (Variables|/Script/Engine.Character|GetMesh _returnvalue) "/Game/Assets/Animations/Bear/Bear_IdleAnim.Bear_IdleAnim" true)))))))

(fn RunTimer
  (Variables|Default|SetSeconds (- (Variables|Default|GetSeconds) 1))
  (if (< (Variables|Default|GetSeconds) 0)
    (Variables|Default|SetMinutes (Variables|Default|GetMinutes))
    (Variables|Default|SetSeconds (Variables|Default|GetSeconds)))
  (if (== (Variables|Default|GetSeconds) 0)
    (if (== (Variables|Default|GetMinutes) 0)
      (Utilities|FlowControl|DoOnce false
        (:Completed
          (Variables|Default|SetRoundOneComplete true)
          (if (Variables|Default|GetRoundOneComplete)
            (CallFunction|RoundTwo)))))))

(fn RunTimerTwo
  (if (Variables|Default|GetRoundOneComplete)
    (Variables|Default|SetRoundTwoSeconds (- (Variables|Default|GetRoundTwoSeconds) 1))
    (if (< (Variables|Default|GetRoundTwoSeconds) 0)
      (Variables|Default|SetRoundTwoMinutes (Variables|Default|GetRoundTwoMinutes))
      (Variables|Default|SetRoundTwoSeconds (Variables|Default|GetRoundTwoSeconds)))
    (if (== (Variables|Default|GetRoundTwoSeconds) 0)
      (if (== (Variables|Default|GetRoundTwoMinutes) 0)
        (Utilities|FlowControl|DoOnce false
          (:Completed
            (Variables|Default|SetRoundTwoComplete true)
            (if (Variables|Default|GetRoundTwoComplete)
              (CallFunction|RoundThree))))))))

(fn RunTimerThree
  (if (Variables|Default|GetRoundTwoComplete)
    (Variables|Default|SetRoundThreeSeconds (- (Variables|Default|GetRoundThreeSeconds) 1))
    (if (< (Variables|Default|GetRoundThreeSeconds) 0)
      (Variables|Default|SetRoundThreeMinutes (Variables|Default|GetRoundThreeMinutes))
      (Variables|Default|SetRoundThreeSeconds (Variables|Default|GetRoundThreeSeconds)))
    (if (== (Variables|Default|GetRoundThreeSeconds) 0)
      (if (== (Variables|Default|GetRoundThreeMinutes) 0)
        (Utilities|FlowControl|DoOnce false
          (:Completed
            (Variables|Default|SetRoundThreeComplete true)
            (if (Variables|Default|GetRoundThreeComplete)
              _)))))))